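; BP_Hole_wall is a wall-hole actor with two mesh ends that launches a rock when play begins.
; The construction script turns HoleWallStart toward the HoleWallEnd position and adds a static mesh there facing back at the start.
; On BeginPlay it spawns a BP_Rock offset from its Arrow component, enables physics, and fires it along the arrow with a mass-independent impulse.
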(event `self.ReceiveBeginPlay`
  (bind _returnvalue (`SceneComponent.K2_GetComponentToWorld` (`self.Arrow`)))
  (bind _returnvalue_2 (`|SpawnActorFromClass` "/Game/Miyazato/BP_Rock.BP_Rock_C" (`KismetMathLibrary.MakeTransform` (`KismetMathLibrary.TransformLocation` _returnvalue (100.0 0.0 -100.0)) (.rotation _returnvalue) (.scale _returnvalue)) "Undefined" "OverrideRootScale" null null))
  (bind _rock (`/Game/Miyazato/BP_Rock.Rock` _returnvalue_2))
  (`PrimitiveComponent.SetSimulatePhysics` _rock true)
  (`PrimitiveComponent.AddImpulse` _rock (`KismetMathLibrary.TransformDirection` _returnvalue (1000.0 0.0 0.0)) "None" true))

(fn `UserConstructionScript`
  (bind _holewallend (`self.HoleWallEnd`))
  (bind _holewallstart (`self.HoleWallStart`))
  (bind _relativelocation (`SceneComponent.RelativeLocation` _holewallstart))
  (`SceneComponent.K2_SetRelativeRotation` _holewallstart (`KismetMathLibrary.FindLookAtRotation` _relativelocation _holewallend) false false)
  (`AddComponent|NODE_AddStaticMeshComponent-1` :`RelativeTransform` (`KismetMathLibrary.MakeTransform` _holewallend (`KismetMathLibrary.FindLookAtRotation` _holewallend _relativelocation))))